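; Lift actor that moves a cabin between evenly spaced floors, with an instanced shaft built at BeginPlay.
; The construction script previews floor positions with instanced meshes, which are removed when play starts.
; UpdateLocationLift eases the cabin toward CurrentFloor's height, driven by Tick, which switches off on arrival, or by a looping timer that UpdateLift toggles.
; LiftDebug picks a random floor and enables Tick.
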(event Custom|UpdateLift
  (if (not (Utilities|Time|IsTimerActivebyHandle (Variables|Default|GetEvent_UpdateLocation)))
    (bind _returnvalue (Utilities|Time|SetTimerbyFunctionName 0 "UpdateLocationLift" 0.01 true))
    (Variables|Default|SetEvent_UpdateLocation _returnvalue)
    (else
      (Utilities|Time|ClearandInvalidateTimerbyHandle (Variables|Default|GetEvent_UpdateLocation)))))

(event EventBeginPlay
  (bind _returnvalue (Transformation|GetActorLocation))
  (CallFunction|RemoveConstructionViewer)
  (Actor|Tick|SetActorTickEnabled false)
  (for _index (range 1 (Variables|Default|GetNumberFloor))
    (Components|InstancedStaticMesh|AddInstance (Variables|Default|GetLiftShaft) (Math|Transform|MakeTransform (Math|Vector|MakeVector (.x _returnvalue) (.y _returnvalue) (+ (.z _returnvalue) (* (Variables|Default|GetDistance) _index))) "0.000000,0.000000,0.000000") true)))

(event EventLiftDebug
  (Variables|Default|SetCurrentFloor (Math|Random|RandomIntegerinRange 0 (Variables|Default|GetNumberFloor)))
  (Actor|Tick|SetActorTickEnabled true))

(event EventTick
  (params (DeltaSeconds :type Float%20%28single-precision%29))
  (CallFunction|UpdateLocationLift))

(fn ConstructionScript
  (bind _returnvalue (Transformation|GetActorLocation))
  (Variables|Default|GetConstructViewer
    (:then
      (for _index (range 0 (Variables|Default|GetNumberFloor))
        (Components|InstancedStaticMesh|AddInstance (Variables|Default|GetConstructViewer) (Math|Transform|MakeTransform (Math|Vector|MakeVector (.x _returnvalue) (.y _returnvalue) (+ (.z _returnvalue) (* (Variables|Default|GetDistance) _index))) "90.000000,0.000000,0.000000" "0.500000,0.500000,0.500000") true)))
    (:else)))

(fn RemoveConstructionViewer
  (bind _constructviewer (Variables|Default|GetConstructViewer))
  (for _index (range 0 (Components|InstancedStaticMesh|GetInstanceCount _constructviewer))
    (Class|InstancedStaticMeshComponent|RemoveInstance _constructviewer _index))
  (Components|DestroyComponent _constructviewer))

(fn UpdateLocationLift
  (bind _lift (Variables|Default|GetLIFT))
  (bind _relativelocation (Variables|/Script/Engine.SceneComponent|GetRelativeLocation _lift))
  (if (not (Math|Float|NearlyEqual(Float) (.z (Variables|/Script/Engine.SceneComponent|GetRelativeLocation (Variables|Default|GetLIFT))) (* (Variables|Default|GetDistance) (Variables|Default|GetCurrentFloor)) 0.5))
    (Transformation|SetRelativeLocation _lift (Math|Vector|MakeVector (.x _relativelocation) (.y _relativelocation) (Math|Interpolation|FInterpTo (.z _relativelocation) (* (Variables|Default|GetDistance) (Variables|Default|GetCurrentFloor)) (Utilities|Time|GetWorldDeltaSeconds) (Variables|Default|GetSpeedElevator))) false false)
    (else
      (Actor|Tick|SetActorTickEnabled false))))